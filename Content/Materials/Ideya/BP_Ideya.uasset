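; Ideya actor that trails the player's pawn and exposes a Flashing toggle on its Niagara effect.
; Each Tick adds a distance-based velocity toward FollowTarget to a capped Speed, then offsets the actor without sweeping.
; BeginFollowPlayer targets the controlled pawn, falling back to player pawn 0, and binds to gameplay state changes to retarget on Visitor, keeping the Ideya after Flight.
; ClearFollowTarget drops the target and unbinds.
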(event `self.ReceiveTick`
  (params (DeltaSeconds :type "Float (single-precision)"))
  (bind _returnvalue (`self.K2_GetActorLocation`))
  ;[1 1 1] Add Force towards Follow Target
  (bind _follow_target (`self.Follow Target`)
    (:`then`
      (bind _returnvalue_2 (`self.K2_GetActorLocation` _follow_target))
      (bind _output_get (set `self.Speed` (`KismetMathLibrary.ClampVectorSize` (+ (`self.Speed`) (* (`KismetMathLibrary.Conv_RotatorToVector` (`KismetMathLibrary.FindLookAtRotation` _returnvalue _returnvalue_2)) (`KismetMathLibrary.MultiplyMultiply_FloatFloat` (`KismetMathLibrary.Vector_Distance` _returnvalue _returnvalue_2) 2.0) 0.05)) 0.0 1500.0)))
      (`self.K2_AddActorWorldOffset` (* _output_get (`GameplayStatics.GetWorldDeltaSeconds`))))
    (:`else`)))

(event `ClearFollowTarget`
  (set `self.Follow Target` null)
  (remove `/Game/ThirdPerson/Blueprints/BP_GameplayController.OnGameplayStateChanged` (stale `RefollowPlayer` _asbp_gameplay_controller) (delegate `RefollowPlayer`)))

(event `RefollowPlayer`
  (params (NewGameplayState :type "/Game/ThirdPerson/Blueprints/GameplayState Enum" :default "NewEnumerator0"))
  ;[0.6158 0.3512 1] Follow the player
  (switch `/Game/ThirdPerson/Blueprints/GameplayState` NewGameplayState ; If the player gets kicked out of Flight (with an ideya following)\nthe player should retain the ideya into the visitor state.
    (:`NewEnumerator0`
      (bind _asbp_gameplay_controller (cast `/Game/ThirdPerson/Blueprints/BP_GameplayController` (`GameplayStatics.GetPlayerController` 0) :!label _label)
        (:`then`
          (set `self.Follow Target` (`Controller.K2_GetPawn` _asbp_gameplay_controller))
          (add `/Game/ThirdPerson/Blueprints/BP_GameplayController.OnGameplayStateChanged` _asbp_gameplay_controller (delegate `RefollowPlayer`)))
        (:`CastFailed`
          (set `self.Follow Target` (`GameplayStatics.GetPlayerPawn` 0)))))))

(event `BeginFollowPlayer`
  ;[0.6158 0.3512 1] Follow the player
  (goto _label))

(fn `SetIdeyaFlashing`
  (params (Flashing :type Boolean))
  (bind _output_get (set `self.Flashing` Flashing))
  (`NiagaraComponent.SetVariableBool` (`self.NS_Ideya`) "Flashing" _output_get))

(fn `UserConstructionScript`
  (`self.SetIdeyaFlashing` (`self.Flashing`)))